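; Crunch Classic enemy variant whose Blueprint supplies the enemy's combat UI: health bar, boss bar and damage numbers.
; The health bar widget component binds to the enemy and starts hidden, while show/hide events toggle it.
; A boss bar is created on the viewport when shown and removed when hidden.
; Hits spawn animated, headshot-aware damage popups at the projected screen position, passed to StoreHitWidget with their world location.
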(event `self.ReceiveBeginPlay`
  (bind _returnvalue (`WidgetComponent.GetUserWidgetObject` (`self.Health Bar`)))
  (bind _asbp_enemy_health_bar (cast `/Game/Gunster/Enemy/HUD/BP_EnemyHealthBar` _returnvalue))
  (set `/Game/Gunster/Enemy/HUD/BP_EnemyHealthBar.Enemy` self _asbp_enemy_health_bar)
  (`Widget.SetVisibility` _returnvalue "Hidden"))

(event `self.ShowBossHealthBar`
  (bind _returnvalue (`|CreateWidget` "/Game/Gunster/Enemy/HUD/BP_BossHealthBar.BP_BossHealthBar_C" (`GameplayStatics.GetPlayerController` 0)))
  (bind _output_get (set `self.CurrentBossHealthBar_0` _returnvalue))
  (set `/Game/Gunster/Enemy/HUD/BP_BossHealthBar.Enemy` self _returnvalue)
  (`UserWidget.AddToViewport` _returnvalue 0)
  (`Widget.SetVisibility` _output_get "Visible"))

(event `self.ShowHealthBar`
  (`parent.ShowHealthBar`)
  (`Widget.SetVisibility` (`WidgetComponent.GetUserWidgetObject` (`self.Health Bar`)) "Visible"))

(event `self.HideBossHealthBar`
  (bind _currentbosshealthbar_0 (`self.CurrentBossHealthBar_0`))
  (`/Engine/EditorBlueprintResources/StandardMacros.IsValid` _currentbosshealthbar_0
    (:`Is Valid`
      (`Widget.RemoveFromParent` _currentbosshealthbar_0))))

(event `self.HideHealthBar`
  (`Widget.SetVisibility` (`WidgetComponent.GetUserWidgetObject` (`self.Health Bar`)) "Hidden"))

(event `self.ShowHitDamageAmount`
  (params (Damage :type "Float (single-precision)") (HitLocation :type "Vector Structure") (bIsHeadShot :type Boolean))
  (bind _returnvalue (`|CreateWidget` "/Game/Gunster/Enemy/HUD/BP_HitDamage.BP_HitDamage_C"))
  (set `/Game/Gunster/Enemy/HUD/BP_HitDamage.bIsHeadShot` bIsHeadShot _returnvalue)
  (`UserWidget.AddToViewport` _returnvalue 0)
  (`UserWidget.SetPositionInViewport` _returnvalue (`GameplayStatics.ProjectWorldToScreen` (`GameplayStatics.GetPlayerController` 0) HitLocation) true)
  (`self.StoreHitWidget` _returnvalue HitLocation)
  (set `/Game/Gunster/Enemy/HUD/BP_HitDamage.DamageAmount` (`KismetTextLibrary.Conv_DoubleToText` Damage "HalfToEven") _returnvalue)
  (`UserWidget.PlayAnimation` _returnvalue (`/Game/Gunster/Enemy/HUD/BP_HitDamage.DamageAmountPopUp` _returnvalue) 0.0 1 "Forward" 1.0 false))

(fn `UserConstructionScript`)