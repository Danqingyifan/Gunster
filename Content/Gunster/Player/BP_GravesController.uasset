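; Player controller for the Graves character that draws a dynamic four-part crosshair for the local player.
; A DrawCrossHair event takes the screen size and draws only while the controlled BP_Graves is aiming and not reloading.
; Top, bottom, left and right textures are drawn through the CrossHair reference around a point slightly above center, pushed outward by base spread times a live spread multiplier.
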(event `Event DrawCrossHair`
  (params (SizeX :type Integer) (SizeY :type Integer))
  (bind _returnvalue (`self.GetCrossHairSpreadMultiplier`))
  (bind _crosshair (`self.CrossHair`))
  ;[1 1 1] Draw CrossHair
  (if (`self.IsLocalController`)
    (bind _asbp_graves (cast `/Game/Gunster/Player/BP_Graves` (`self.K2_GetPawn`)))
    (if (`GunsterCharacter.bIsAiming` _asbp_graves)
      ;;[1 1 1] Update SpreadMultiplier
      (set `self.CrossHairSpreadMultiplier` (`self.GetCrossHairSpreadMultiplier`))
      (if (not (`GunsterCharacter.bIsReloading` _asbp_graves))
        (bind _output_get (set `self.Viewport Center` (`KismetMathLibrary.MakeVector2D` (+ (`KismetMathLibrary.Conv_IntToDouble` (/ SizeX 2)) 0.0) (- (`KismetMathLibrary.Conv_IntToDouble` (/ SizeY 2)) 50.0))))
        (`HUD.DrawTexture` _crosshair "/Game/Assets/Texture/Icons/Crosshairs/Crosshair_Quad_9_Top.Crosshair_Quad_9_Top" (`KismetMathLibrary.BreakVector2D` _output_get) (- (`.Y` (`KismetMathLibrary.BreakVector2D` _output_get)) (* (`self.CrossHairSpreadBase`) _returnvalue)) 64.0 64.0 0.0 0.0 1.0 1.0 (struct :`R` 1.0 :`G` 1.0 :`B` 1.0 :`A` 1.0) "BLEND_Translucent" 1.0 false 0.0 (0.0 0.0))
        (`HUD.DrawTexture` _crosshair "/Game/Assets/Texture/Icons/Crosshairs/Crosshair_Quad_9_Bottom.Crosshair_Quad_9_Bottom" (`KismetMathLibrary.BreakVector2D` _output_get) (+ (`.Y` (`KismetMathLibrary.BreakVector2D` _output_get)) (* (`self.CrossHairSpreadBase`) _returnvalue)) 64.0 64.0 0.0 0.0 1.0 1.0 (struct :`R` 1.0 :`G` 1.0 :`B` 1.0 :`A` 1.0) "BLEND_Translucent" 1.0 false 0.0 (0.0 0.0))
        (`HUD.DrawTexture` _crosshair "/Game/Assets/Texture/Icons/Crosshairs/Crosshair_Quad_9_Left.Crosshair_Quad_9_Left" (- (`KismetMathLibrary.BreakVector2D` _output_get) (* (`self.CrossHairSpreadBase`) _returnvalue)) (`.Y` (`KismetMathLibrary.BreakVector2D` _output_get)) 64.0 64.0 0.0 0.0 1.0 1.0 (struct :`R` 1.0 :`G` 1.0 :`B` 1.0 :`A` 1.0) "BLEND_Translucent" 1.0 false 0.0 (0.0 0.0))
        (`HUD.DrawTexture` _crosshair "/Game/Assets/Texture/Icons/Crosshairs/Crosshair_Quad_9_Right.Crosshair_Quad_9_Right" (+ (`KismetMathLibrary.BreakVector2D` _output_get) (* (`self.CrossHairSpreadBase`) _returnvalue)) (`.Y` (`KismetMathLibrary.BreakVector2D` _output_get)) 64.0 64.0 0.0 0.0 1.0 1.0 (struct :`R` 1.0 :`G` 1.0 :`B` 1.0 :`A` 1.0) "BLEND_Translucent" 1.0 false 0.0 (0.0 0.0))))))

(fn `UserConstructionScript`)